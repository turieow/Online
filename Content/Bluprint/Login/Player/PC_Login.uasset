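; PC_Login is the player controller for the login screen.
; On BeginPlay it creates the WBP_Login widget, adds it to the viewport, shows the mouse cursor and switches to UI-only input.
; Pressing Escape calls DestroySessionMessage on the game instance, passing itself.
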(event `self.ReceiveBeginPlay`
  (bind _returnvalue (`GameplayStatics.GetPlayerController` 0))
  (`self.E_CreateLoginUI`)
  (set `PlayerController.bShowMouseCursor` true _returnvalue)
  (`WidgetBlueprintLibrary.SetInputMode_UIOnlyEx` _returnvalue null))

(event `E_CreateLoginUI`
  (bind _returnvalue (`|CreateWidget` "/Game/Bluprint/Login/UI/WBP_Login.WBP_Login_C" self))
  (bind _output_get (set `self.LoginUI` _returnvalue))
  (`UserWidget.AddToViewport` _output_get 0))

(event `Key|Escape`
  (params (Key :type "Key Structure"))
  (:`Pressed`
    (message `/Game/Bluprint/Interface/BPI_ToGameInstance.DestroySession` (`GameplayStatics.GetGameInstance`) self)))

(fn `UserConstructionScript`)