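; BP_GhostManager is a manager Blueprint that gathers the level's BP_Ghost actors and keeps a running Score.
; BeginPlay caches every ghost in the Ghosts array, which nothing else in its graphs uses.
; RoS_AddScore passes points to MC_AddScore (named as a server-to-multicast pair) to increase Score.
; It then copies the total to player controller 0's PlayerState through the ICopyScoreMessage interface call.
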(event `self.ReceiveBeginPlay`
  (bind _outactors (`GameplayStatics.GetAllActorsOfClass` "/Game/Bluprint/Main/Player/Ghost/BP_Ghost.BP_Ghost_C"))
  (set `self.Ghosts` _outactors))

(event `RoS_AddScore`
  (params (AddScore :type Integer))
  (`self.MC_AddScore` AddScore)
  (`self.E_CopyDataToPlayerState`))

(event `MC_AddScore`
  (params (AddScore :type Integer))
  (set `self.Score` (+ (`self.Score`) AddScore)))

(event `E_CopyDataToPlayerState`
  (message `/Game/Bluprint/Main/Player/BPI_ToPlayerState.ICopyScore` (`Controller.PlayerState` (`GameplayStatics.GetPlayerController` 0)) (`self.Score`)))

(fn `UserConstructionScript`)