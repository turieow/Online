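; Player controller that manages the on-screen UI for the Matching and Main game phases.
; BeginPlay hides the cursor, sets game-only input and creates the matching widget.
; Game-status interface events route state changes: finalising Matching removes its widget and initialising Main creates the main widget.
; RoC-prefixed events handle widget creation and removal; Matching initialisation is empty and main UI removal is never called here.
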(event `self.ReceiveBeginPlay`
  (`self.E_InitPlayerController`))

(event `E_InitPlayerController`
  (set `self.bShowMouseCursor` false)
  (`WidgetBlueprintLibrary.SetInputMode_GameOnly` self)
  (`self.RoC_CreateMatchingUI`))

(event `/Game/Bluprint/Main/Player/BPI_ToPlayerController.IInitGameStatus`
  (params (newState :type "/Game/Bluprint/Enum/En_GameStatus Enum" :default "NewEnumerator0"))
  ;[1 1 1] ゲームのステータス　初期化
  (switch `/Game/Bluprint/Enum/En_GameStatus` newState
    (:`NewEnumerator0`
      (`self.E_InitMatchingState`))
    (:`NewEnumerator1`
      (`self.E_InitMainState`))))

(event `/Game/Bluprint/Main/Player/BPI_ToPlayerController.IFinaliseGameStatus`
  (params (beforestate :type "/Game/Bluprint/Enum/En_GameStatus Enum" :default "NewEnumerator0"))
  ;[1 1 1] ゲームのステータス　ファイナライズ
  (switch `/Game/Bluprint/Enum/En_GameStatus` beforestate
    (:`NewEnumerator0`
      (`self.E_FinaliseMatchingState`))))

(event `E_InitMatchingState`)

(event `E_FinaliseMatchingState`
  (`self.RoC_RemoveMatchingUI`))

(event `RoC_CreateMatchingUI`
  ;[1 1 1] マッチングＵＩを作成
  (bind _returnvalue (`|CreateWidget` "/Game/Bluprint/Matching/UI/WBP_Matching.WBP_Matching_C" (`GameplayStatics.GetPlayerController` 0)))
  (bind _output_get (set `self.MatchingUI` _returnvalue))
  (`UserWidget.AddToViewport` _output_get 0))

(event `RoC_RemoveMatchingUI`
  ;[1 1 1] マッチングＵＩ Remove
  (bind _matchingui (`self.MatchingUI`)
    (:`then`
      (`Widget.RemoveFromParent` _matchingui))
    (:`else`)))

(event `E_InitMainState`
  (`self.RoC_CreateMainUI`))

(event `RoC_CreateMainUI`
  ;[1 1 1] マッチングＵＩを作成
  (bind _returnvalue (`|CreateWidget` "/Game/Bluprint/Main/UI/WBP_Main.WBP_Main_C" (`GameplayStatics.GetPlayerController` 0)))
  (bind _output_get (set `self.MainUI` _returnvalue))
  (`UserWidget.AddToViewport` _output_get 0))

(event `RoC_RemoveMainUI`
  ;[1 1 1] RemoveMainUI
  (bind _mainui (`self.MainUI`)
    (:`then`
      (`Widget.RemoveFromParent` _mainui))
    (:`else`)))

(fn `UserConstructionScript`)