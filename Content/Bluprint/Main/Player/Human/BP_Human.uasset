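; BP_Human is the human player Blueprint, holding a replicated-by-RPC score.
; The AddScore interface event adds to the current score and sends the total through a SetScore RPC pair, named as run-on-server then multicast, which assigns it.
; It then passes Score to player controller 0's PlayerState through a CopyScoreMessage interface call.
; The construction script only calls its parent.
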(event `/Game/Bluprint/Main/Player/BPI_ToPlayer.IAddScore`
  (params (AddScore :type Integer))
  (`self.RoS_SetScore` (+ AddScore (`self.Score`)))
  (message `/Game/Bluprint/Main/Player/BPI_ToPlayerState.ICopyScore` (`Controller.PlayerState` (`GameplayStatics.GetPlayerController` 0)) (`self.Score`)))

(event `RoS_SetScore`
  (params (Score :type Integer))
  ;[1 1 1] スコア設定
  (`self.MC_SetScore` Score))

(event `MC_SetScore`
  (params (Score :type Integer))
  ;[1 1 1] スコア設定
  (set `self.Score` Score))

(fn `UserConstructionScript`
  (`parent.UserConstructionScript`))