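; Matchmaking game mode that holds joining players until the match is full, then moves the server to the main map.
; PostLogin stores each controller and compares the GameState player count to a maximum read from the game instance.
; On a match, it waits briefly and issues a servertravel console command for L_Main.
; Debug prints show the server's player count each tick; alternative travel branches are left disconnected.
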(event `self.HandleStartingNewPlayer`
  (params (NewPlayer :type "PlayerController Object Reference"))
  (`KismetSystemLibrary.PrintString` "Hello"))

(event `self.K2_PostLogin`
  (params (NewPlayer :type "PlayerController Object Reference"))
  (`KismetArrayLibrary.Array_Add` (`self.PlayerControllers`) NewPlayer)
  (bind _num (message `/Game/Bluprint/Interface/BPI_ToGameInstance.GetMaxPlayerNum` (`GameplayStatics.GetGameInstance`)))
  (if (== _num (`KismetArrayLibrary.Array_Length` (`GameStateBase.PlayerArray` (`GameplayStatics.GetGameState`))))
    (`KismetSystemLibrary.PrintString` "マッチング完了")
    (`KismetSystemLibrary.Delay` 1.0)
    (`KismetSystemLibrary.ExecuteConsoleCommand` (`KismetStringLibrary.Concat_StrStr` "servertravel" "/Game/Map/L_Main.L_Main'") null)
    (`KismetSystemLibrary.PrintString` "travel" true true (struct :`R` 1.0 :`B` 0.218701 :`A` 1.0))))

(event `self.ReceiveTick`
  (params (DeltaSeconds :type "Float (single-precision)"))
  (`/Engine/EditorBlueprintResources/ActorMacros.Switch Has Authority`
    (:`Authority`
      (`KismetSystemLibrary.PrintString` (`KismetStringLibrary.Conv_IntToString` (`KismetArrayLibrary.Array_Length` (`GameStateBase.PlayerArray` (`GameplayStatics.GetGameState`)))) true true (struct :`G` 0.66 :`B` 1.0 :`A` 1.0) 0.0))))

(fn `UserConstructionScript`)